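; Remote-control input object that converts mouse movement and key events to and from JSON so another instance's input can be replayed locally.
; Builder functions write a message type plus mouse position with viewport and screen sizes, or key name with input event.
; ProcessRCMessage parses incoming strings and dispatches by type to SetMousePosition, passing the sender's dimensions, or to InputKey.
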(event Custom|ProcessRCMessage
  (params (JsonStr :type String))
  (CallFunction|ProcessJsonString JsonStr))

(event Custom|CustomEvent_0
  (params (KeyName :type Name) (InputEvent :type EInputEvent%20Enum :default "IE_Pressed"))
  (Class|RCInputObj|InputKey KeyName InputEvent))

(fn MakeMouseMoveJsonString
  (params (X :type Float%20%28single-precision%29) (Y :type Float%20%28single-precision%29))
  (bind (_x _y) (Class|RCInputObj|GetScreenSize))
  (bind _playercontroller (Variables|Default|GetPlayerController))
  (bind (_sizex _sizey) (HUD|GetViewportSize _playercontroller))
  (bind _output_get (LocalVariables|SetJsonObj (Class|JsonObjectFactory|ConstructJsonObject)))
  (Class|JsonObj|SetIntegerField _output_get "Type" (Math|Conversions|ToInteger(Byte) (LocalVariables|GetMessageType)))
  (bind _output_get_2 (LocalVariables|SetMouseInfoObj (Class|JsonObjectFactory|ConstructJsonObject)))
  (Class|JsonObj|SetNumberField _output_get_2 "X" X)
  (Class|JsonObj|SetNumberField _output_get_2 "Y" Y)
  (Class|JsonObj|SetNumberField _output_get_2 "ViewportSizeX" (Math|Conversions|ToFloat(Integer) _sizex))
  (Class|JsonObj|SetNumberField _output_get_2 "ViewportSizeY" (Math|Conversions|ToFloat(Integer) _sizey))
  (Class|JsonObj|SetNumberField _output_get_2 "ScreenSizeX" (Math|Conversions|ToFloat(Integer) _x))
  (Class|JsonObj|SetNumberField _output_get_2 "ScreenSizeY" (Math|Conversions|ToFloat(Integer) _y))
  (Class|JsonObj|SetObjectField (LocalVariables|GetJsonObj) "MouseInfo" (LocalVariables|GetMouseInfoObj))
  (return (.JsonStr (Class|JsonObj|AsJsonStr (LocalVariables|GetJsonObj))) (.ReturnValue (Class|JsonObj|AsJsonStr (LocalVariables|GetJsonObj)))))

(fn MakeKeyInputJsonString
  (params (KeyName :type Name) (InputEvent :type EInputEvent%20Enum :default "IE_Pressed"))
  (bind _output_get (LocalVariables|SetJsonObj (Class|JsonObjectFactory|ConstructJsonObject)))
  (Class|JsonObj|SetIntegerField _output_get "Type" (Math|Conversions|ToInteger(Byte) (LocalVariables|GetMessageType)))
  (bind _output_get_2 (LocalVariables|SetKeyInfoObj (Class|JsonObjectFactory|ConstructJsonObject)))
  (Class|JsonObj|SetStringField _output_get_2 "KeyName" (Utilities|String|ToString(Name) KeyName))
  (Class|JsonObj|SetIntegerField _output_get_2 "InputEvent" (Math|Conversions|ToInteger(Byte) InputEvent))
  (Class|JsonObj|SetObjectField (LocalVariables|GetJsonObj) "KeyInfo" (LocalVariables|GetKeyInfoObj))
  (return (.JsonStr (Class|JsonObj|AsJsonStr (LocalVariables|GetJsonObj))) (.ReturnValue (Class|JsonObj|AsJsonStr (LocalVariables|GetJsonObj)))))

(fn ProcessJsonString
  (params (JsonStr :type String))
  (bind _returnvalue (Class|JsonObjectFactory|ConstructJsonObjectfromJsonString JsonStr))
  (Utilities|IsValid _returnvalue
    (:Is%20Valid
      (bind _output_get (LocalVariables|SetJsonObj _returnvalue))
      (switch Utilities|FlowControl|Switch|SwitchonBPE_RCInput_MessageType (Utilities|Enum|ByteToEnumBPE_RCInput_MessageType (Math|Conversions|ToByte(Integer) (.OutInteger (Class|JsonObj|GetIntegerField _output_get "Type"))))
        (:NewEnumerator0
          (bind _returnvalue_2 (Class|RCInputObj|SetMousePosition (Math|Float|Truncate (.OutNumber (Class|JsonObj|GetNumberField (Class|JsonObj|GetObjectField (LocalVariables|GetJsonObj) "MouseInfo") "X"))) (Math|Float|Truncate (.OutNumber (Class|JsonObj|GetNumberField (Class|JsonObj|GetObjectField (LocalVariables|GetJsonObj) "MouseInfo") "Y"))) (Math|Float|Truncate (.OutNumber (Class|JsonObj|GetNumberField (Class|JsonObj|GetObjectField (LocalVariables|GetJsonObj) "MouseInfo") "ViewportSizeX"))) (Math|Float|Truncate (.OutNumber (Class|JsonObj|GetNumberField (Class|JsonObj|GetObjectField (LocalVariables|GetJsonObj) "MouseInfo") "ViewportSizeY"))) (Math|Float|Truncate (.OutNumber (Class|JsonObj|GetNumberField (Class|JsonObj|GetObjectField (LocalVariables|GetJsonObj) "MouseInfo") "ScreenSizeX"))) (Math|Float|Truncate (.OutNumber (Class|JsonObj|GetNumberField (Class|JsonObj|GetObjectField (LocalVariables|GetJsonObj) "MouseInfo") "ScreenSizeY")))))
          (return _returnvalue_2))
        (:NewEnumerator2
          (bind _returnvalue_3 (Class|RCInputObj|InputKey (Utilities|String|StringToName (.OuStr (Class|JsonObj|GetStringField (Class|JsonObj|GetObjectField (LocalVariables|GetJsonObj) "KeyInfo") "KeyName"))) (Utilities|Enum|ByteToEnumEInputEvent (Math|Conversions|ToByte(Integer) (.OutInteger (Class|JsonObj|GetIntegerField (Class|JsonObj|GetObjectField (LocalVariables|GetJsonObj) "KeyInfo") "InputEvent"))))))
          (return _returnvalue_3))))))